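; BP_ShotgunAmmo is a pickup that replenishes the player's shotgun ammo.
; When its Box component begins overlapping the actor held in PlayerRef, it adds a random amount of shells, clamps the total to the player's maximum and destroys itself.
; PlayerRef is not assigned in these graphs, and the BeginPlay, Tick and actor overlap events are disabled stubs.
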(event `self.Box.OnComponentBeginOverlap`
  (params (OverlappedComponent :type "PrimitiveComponent Object Reference") (OtherActor :type "Actor Object Reference") (OtherComp :type "PrimitiveComponent Object Reference") (OtherBodyIndex :type Integer) (bFromSweep :type Boolean) (SweepResult :type "HitResult Structure (by ref)"))
  (bind _playerref (`self.PlayerRef`))
  (if (== OtherActor (`self.PlayerRef`))
    (set `/Game/FirstPerson/Blueprints/BPFirstPersonCharacter.ShotgunAmmo` (`KismetMathLibrary.Clamp` (+ (`/Game/FirstPerson/Blueprints/BPFirstPersonCharacter.ShotgunAmmo` _playerref) (`KismetMathLibrary.RandomIntegerInRange` 10 25)) 0 (`/Game/FirstPerson/Blueprints/BPFirstPersonCharacter.MaxShotgunAmmo` (`self.PlayerRef`))) _playerref)
    (`self.K2_DestroyActor`)))

(fn `UserConstructionScript`
  (`parent.UserConstructionScript`))