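; BP_Bounds is an out-of-bounds volume that kills the first-person character if it stays inside the trigger too long.
; When the character begins overlapping BoundsTrigger, it sets an OutOfBounds flag, shows the WB_OutOfBounds warning widget and waits five seconds.
; If the flag is still set after the delay, it applies lethal damage.
; Ending the overlap clears the flag and removes the widget.
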(event `self.Bounds Trigger.OnComponentBeginOverlap`
  (params (OverlappedComponent :type "PrimitiveComponent Object Reference") (OtherActor :type "Actor Object Reference") (OtherComp :type "PrimitiveComponent Object Reference") (OtherBodyIndex :type Integer) (bFromSweep :type Boolean) (SweepResult :type "HitResult Structure (by ref)"))
  (bind _asbpfirst_person_character (cast `/Game/FirstPerson/Blueprints/BPFirstPersonCharacter` OtherActor))
  (set `self.OutOfBounds` true)
  (bind _returnvalue (`|CreateWidget` "/Game/WB_OutOfBounds.WB_OutOfBounds_C"))
  (bind _output_get (set `self.Widget` _returnvalue))
  (`UserWidget.AddToViewport` _output_get 0)
  (`KismetSystemLibrary.Delay` 5.0)
  (if (`self.OutOfBounds`)
    (`/Game/FirstPerson/Blueprints/BPFirstPersonCharacter.TakeDamage` _asbpfirst_person_character 10000.0 null)))

(event `self.Bounds Trigger.OnComponentEndOverlap`
  (params (OverlappedComponent :type "PrimitiveComponent Object Reference") (OtherActor :type "Actor Object Reference") (OtherComp :type "PrimitiveComponent Object Reference") (OtherBodyIndex :type Integer))
  (cast `/Game/FirstPerson/Blueprints/BPFirstPersonCharacter` OtherActor)
  (set `self.OutOfBounds` false)
  (bind _widget (`self.Widget`)
    (:`then`
      (`Widget.RemoveFromParent` _widget)
      (set `self.Widget` null))
    (:`else`)))

(fn `UserConstructionScript`)