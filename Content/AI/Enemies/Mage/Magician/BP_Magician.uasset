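; BP_Magician is the Magician enemy, which detects the player by sight through a PawnSensing component.
; When it sees the first-person character, it snaps its full rotation toward that character's location.
; It then sets the SensesPlayer Blackboard key to true through its AIC_Magician controller.
; Nothing in this Blueprint clears that key or runs on Tick.
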(event `self.PawnSensing.OnSeePawn`
  (params (Pawn :type "Pawn Object Reference"))
  (bind _asbpfirst_person_character (cast `/Game/FirstPerson/Blueprints/BPFirstPersonCharacter` Pawn))
  (`self.K2_SetActorRotation` (`KismetMathLibrary.FindRelativeLookAtRotation` (`KismetMathLibrary.Conv_VectorToTransform` (`self.K2_GetActorLocation`)) (`self.K2_GetActorLocation` _asbpfirst_person_character)))
  (bind _asaic_magician (cast `/Game/AI/Enemies/Mage/Magician/AIC_Magician` (`self.GetController`)))
  (`BlackboardComponent.SetValueAsBool` (`AIController.Blackboard` _asaic_magician) "SensesPlayer" true))

(fn `UserConstructionScript`
  (`parent.UserConstructionScript`))