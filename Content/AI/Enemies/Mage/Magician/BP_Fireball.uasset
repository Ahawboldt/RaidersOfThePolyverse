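; BP_Fireball is a magician enemy's projectile that explodes when it overlaps any actor not tagged Enemy.
; On impact it spawns the P_Molotov emitter, runs a sphere overlap that ignores all BP_EnemyMaster actors, then destroys itself.
; Each actor found by the overlap applies damage to player 0's BPFirstPersonCharacter, whether or not that actor is the player.
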(event `self.ReceiveActorBeginOverlap`
  (params (OtherActor :type "Actor Object Reference"))
  (bind _returnvalue (`SceneComponent.K2_GetComponentLocation` (`self.Sphere`)))
  (if (not (`self.ActorHasTag` OtherActor "Enemy"))
    (`GameplayStatics.SpawnEmitterAtLocation` "/Game/Realistic_Starter_VFX_Pack_Vol2/Particles/Explosion/P_Molotov.P_Molotov" _returnvalue)
    (bind _outactors (`GameplayStatics.GetAllActorsOfClass` "/Game/AI/Enemies/BP_EnemyMaster.BP_EnemyMaster_C"))
    (bind _outactors_2 (`KismetSystemLibrary.SphereOverlapActors` _returnvalue 150.0 (`|MakeArray` "ObjectTypeQuery3" "ObjectTypeQuery1" "ObjectTypeQuery2" "ObjectTypeQuery4" "ObjectTypeQuery5" "ObjectTypeQuery6" "ObjectTypeQuery7" :!type "EObjectTypeQuery Enum") null _outactors))
    (for _ _outactors_2
      (bind _asbpfirst_person_character (cast `/Game/FirstPerson/Blueprints/BPFirstPersonCharacter` (`GameplayStatics.GetPlayerCharacter` 0)))
      (`/Game/FirstPerson/Blueprints/BPFirstPersonCharacter.TakeDamage` _asbpfirst_person_character 0.5 null))
    (`self.K2_DestroyActor`)))

(fn `UserConstructionScript`)