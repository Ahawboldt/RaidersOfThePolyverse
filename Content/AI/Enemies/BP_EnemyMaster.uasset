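; Base enemy Blueprint that handles damage, death and loot drops.
; TakeDamage passes damage to BPCHealth; when RemoveHealth returns true, the mesh ragdolls, capsule collision turns off and the mesh ignores Visibility traces.
; AmmoDrop and SpawnWeapon then spawn a random ammo type and weapon at AmmoDropLocation.
; Both drops always occur, as every outer ammo roll reaches the spawn and the weapon chance check always passes.
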(event `self.ReceiveBeginPlay`)

(fn `AmmoDrop`
  (bind _returnvalue (`KismetMathLibrary.RandomIntegerInRange` 0 4))
  (bind _returnvalue_2 (`KismetMathLibrary.Conv_VectorToTransform` (`SceneComponent.K2_GetComponentLocation` (`self.AmmoDropLocation`))))
  (switch `int` _returnvalue
    (:`0`
      _)
    (:`1`
      _)
    (:`2`
      _)
    (:`3`
      _)
    (:`4`
      _))
  (switch `int` _returnvalue
    (:`0`
      (`|SpawnActorFromClass` "/Game/Pickups/Ammo/BP_AssaultRifleAmmo.BP_AssaultRifleAmmo_C" _returnvalue_2 "Undefined" "MultiplyWithRoot" null null))
    (:`1`
      (`|SpawnActorFromClass` "/Game/Pickups/Ammo/BP_GrenadeAmmo.BP_GrenadeAmmo_C" _returnvalue_2 "Undefined" "MultiplyWithRoot" null null))
    (:`2`
      (`|SpawnActorFromClass` "/Game/Pickups/Ammo/BP_ShotgunAmmo.BP_ShotgunAmmo_C" _returnvalue_2 "Undefined" "MultiplyWithRoot" null null))
    (:`3`
      (`|SpawnActorFromClass` "/Game/Pickups/Ammo/BP_SMGAmmo.BP_SMGAmmo_C" _returnvalue_2 "Undefined" "MultiplyWithRoot" null null))
    (:`4`
      (`|SpawnActorFromClass` "/Game/Pickups/Ammo/BP_SniperAmmo.BP_SniperAmmo_C" _returnvalue_2 "Undefined" "MultiplyWithRoot" null null))))

(fn `SpawnWeapon`
  (bind _returnvalue (`KismetMathLibrary.Conv_VectorToTransform` (`SceneComponent.K2_GetComponentLocation` (`self.AmmoDropLocation`))))
  (if (<= (`KismetMathLibrary.RandomFloatInRange` 0.0 1.0) 9.0)
    (switch `int` (`KismetMathLibrary.RandomIntegerInRange` 0 3)
      (:`0`
        (`|SpawnActorFromClass` "/Game/Weapons/Weapon_AssaultRifle.Weapon_AssaultRifle_C" _returnvalue "Undefined" "MultiplyWithRoot" null (`self.Instigator`)))
      (:`1`
        (`|SpawnActorFromClass` "/Game/Weapons/Weapon_SMG.Weapon_SMG_C" _returnvalue "Undefined" "MultiplyWithRoot" null null))
      (:`2`
        (`|SpawnActorFromClass` "/Game/Weapons/BP_Shotgun.BP_Shotgun_C" _returnvalue "Undefined" "MultiplyWithRoot" null null))
      (:`3`
        (`|SpawnActorFromClass` "/Game/Weapons/BP_Sniper.BP_Sniper_C" _returnvalue "Undefined" "MultiplyWithRoot" null null)))))

(fn `TakeDamage`
  (params (Amount :type "Float (double-precision)"))
  (returns (Dead :type Boolean))
  (bind _dead (`/Game/FirstPerson/Blueprints/BPC_Health.RemoveHealth` (`self.BPC_Health`) Amount))
  (if _dead
    (`PrimitiveComponent.SetSimulatePhysics` (`self.Mesh`) true)
    (`PrimitiveComponent.SetCollisionEnabled` (`self.CapsuleComponent`) "NoCollision")
    (`PrimitiveComponent.SetCollisionResponseToChannel` (`self.Mesh`) "ECC_Visibility" "ECR_Ignore")
    (`self.AmmoDrop`)
    (`self.SpawnWeapon`)
    (return true)))

(fn `UserConstructionScript`)