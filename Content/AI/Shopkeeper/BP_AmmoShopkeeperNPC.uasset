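; BP_AmmoShopkeeperNPC is a shopkeeper NPC that opens the ammo shop when interacted with.
; Interact plays one of three random greeting sounds, then blends the player camera to the NPC and waits briefly.
; It then creates the W_AmmoShop widget with a reference to itself, switches input to UI only with the cursor shown, and pauses the game.
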(event `/Game/AI/Shopkeeper/BP_InteractInterface.Interact`
  (bind _returnvalue (`GameplayStatics.GetPlayerController` 0))
  (switch `int` (`KismetMathLibrary.RandomIntegerInRange` 0 2)
    (:`0`
      (`GameplayStatics.PlaySound2D` "/Game/AI/Shopkeeper/ShopkeeperAssets/you_again.you_again" 1.0 1.0 0.0 null null))
    (:`1`
      (`GameplayStatics.PlaySound2D` "/Game/AI/Shopkeeper/ShopkeeperAssets/hey_may_I_help.hey_may_I_help" 1.0 1.0 0.0 null null))
    (:`2`
      (`GameplayStatics.PlaySound2D` "/Game/AI/Shopkeeper/ShopkeeperAssets/welcome_0.welcome_0" 1.0 1.0 0.0 null null)))
  (`PlayerController.SetViewTargetWithBlend` (`GameplayStatics.GetPlayerController` 0) self 1.0 "VTBlend_Linear" 0.0 false)
  (`KismetSystemLibrary.Delay` 1.2)
  (bind _returnvalue_2 (`|CreateWidget` "/Game/AI/Shopkeeper/W_AmmoShop.W_AmmoShop_C" null self))
  (`UserWidget.AddToViewport` _returnvalue_2 0)
  (`WidgetBlueprintLibrary.SetInputMode_UIOnlyEx` _returnvalue _returnvalue_2)
  (set `PlayerController.bShowMouseCursor` true _returnvalue)
  (`GameplayStatics.SetGamePaused` true))

(fn `UserConstructionScript`)