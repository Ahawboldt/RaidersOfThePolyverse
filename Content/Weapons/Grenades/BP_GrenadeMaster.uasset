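; Master grenade actor that explodes on a fuse timer and damages what is around it.
; BeginPlay caches the first-person player character and, only if that cast succeeds, starts the timer that calls Explode by name.
; Explode spawns an explosion emitter, then sphere-overlaps pawns and world-static objects to apply damage.
; DestroyActor sits inside the damage loop, so the grenade is destroyed only when something overlaps.
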(event `self.ReceiveBeginPlay`
  (bind _asbpfirst_person_character (cast `/Game/FirstPerson/Blueprints/BPFirstPersonCharacter` (`GameplayStatics.GetPlayerCharacter` 0)))
  (set `self.PlayerRef` _asbpfirst_person_character)
  (`KismetSystemLibrary.K2_SetTimer` null "Explode" (`self.FuseTime`)))

(fn `Explode`
  (`GameplayStatics.SpawnEmitterAtLocation` "/Game/Realistic_Starter_VFX_Pack_Vol2/Particles/Explosion/P_Explosion_Big_A.P_Explosion_Big_A" (`SceneComponent.K2_GetComponentLocation` (`self.Grenade`)))
  (bind _outactors (`KismetSystemLibrary.SphereOverlapActors` (`self.K2_GetActorLocation`) (`self.ExplosionRadius`) (`|MakeArray` "ObjectTypeQuery3" "ObjectTypeQuery1" :!type "EObjectTypeQuery Enum")))
  (for _array_element _outactors
    (`GameplayStatics.ApplyDamage` _array_element (`self.Damage`))
    (`self.K2_DestroyActor`)))

(fn `UserConstructionScript`)