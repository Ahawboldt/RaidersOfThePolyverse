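; Master weapon Blueprint that handles starting clip ammo and procedural recoil motion for its Gun component.
; Construction fills the clip to max, and SetRecoilVariables caches the gun's pitch and X position plus kicked-up, pulled-back targets.
; RecoilAnimation lerps pitch and X by a caller-supplied Alpha, preserving other axes.
; Its pitch lerp starts from PreRecoilRotation, whereas the setup function writes PreRecoilRot.
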(fn `RecoilAnimation`
  (params (Alpha :type "Float (double-precision)"))
  (bind _gun (`self.Gun`))
  (bind _gun_2 (`self.Gun`))
  (bind (_relativerotation_roll _relativerotation_pitch _relativerotation_yaw) (`KismetMathLibrary.BreakRotator` (`SceneComponent.RelativeRotation` _gun)))
  (bind (_relativelocation_x _relativelocation_y _relativelocation_z) (`KismetMathLibrary.BreakVector` (`SceneComponent.RelativeLocation` _gun_2)))
  (`SceneComponent.K2_SetRelativeRotation` _gun (`KismetMathLibrary.MakeRotator` _relativerotation_roll (`KismetMathLibrary.Lerp` (`self.PreRecoilRotation`) (`self.RecoilRotationAmount`) Alpha) _relativerotation_yaw) false false)
  (`SceneComponent.K2_SetRelativeLocation` _gun_2 (`KismetMathLibrary.MakeVector` (`KismetMathLibrary.Lerp` (`self.Pre Recoil Loc`) (`self.RecoilLocationAmount`) Alpha) _relativelocation_y _relativelocation_z) false false))

(fn `SetRecoilVariables`
  (bind (_relativerotation_roll _relativerotation_pitch) (`KismetMathLibrary.BreakRotator` (`SceneComponent.RelativeRotation` (`self.Gun`))))
  (bind _relativelocation_x (`KismetMathLibrary.BreakVector` (`SceneComponent.RelativeLocation` (`self.Gun`))))
  (set `self.PreRecoilRot` _relativerotation_pitch)
  (set `self.RecoilRotationAmount` (+ _relativerotation_pitch (`self.RecoilAmount`)))
  (set `self.Pre Recoil Loc` _relativelocation_x)
  (set `self.RecoilLocationAmount` (+ _relativelocation_x (* (`self.PullBackAmount`) -1.0))))

(fn `UserConstructionScript`
  (set `self.CurrentClipAmmo` (`self.MaxClipAmmo`)))